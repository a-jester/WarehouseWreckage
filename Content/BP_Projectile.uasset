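; Projectile Blueprint that launches itself by physics impulse on its static mesh component.
; LaunchProjectile applies a fixed impulse along the mesh's forward vector as a velocity change, so mass does not affect launch speed.
; PrintYourName prints the object's display name.
; The event graph and construction script are empty, so neither function is called from within this Blueprint.
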(event EventBeginPlay)

(event Collision|EventActorBeginOverlap
  (params (OtherActor :type Actor%20Object%20Reference)))

(event EventTick
  (params (DeltaSeconds :type Float%20%28single-precision%29)))

(fn ConstructionScript)

(fn PrintYourName
  (Development|PrintString (Utilities|GetDisplayName self)))

(fn LaunchProjectile
  (Physics|AddImpulse (Variables|/Script/Engine.StaticMeshActor|GetStaticMeshComponent self) (* (Math|Vector|GetForwardVector (Variables|/Script/Engine.StaticMeshActor|GetStaticMeshComponent self)) 5e+03) "None" true))